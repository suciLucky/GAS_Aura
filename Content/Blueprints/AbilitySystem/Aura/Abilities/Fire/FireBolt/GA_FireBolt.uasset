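; GA_FireBolt is a gameplay ability that casts a fire bolt projectile toward the point under the mouse.
; On activation it commits, gets target data under the mouse and turns the avatar to face that point through an interface.
; It plays the cast montage and waits for a gameplay event, then spawns the projectile from the weapon socket.
; The ability ends when the montage completes, blends out or is stopped.
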(event `self.K2_ActivateAbility`
  (`self.K2_CommitAbility`)
  (bind (_asynctaskproxy _datahandle) (`TargetDataUnderMouse.CreatTargetDataUnderMouse`)
    (:`ValidData`
      (set `self.ProjectileTargetLocation` (`.Location` (`GameplayStatics.BreakHitResult` (`AbilitySystemBlueprintLibrary.GetHitResultFromTargetData` _datahandle))))
      ;[1 1 1] 通过接口调用
      (message `CombatInterface.UpdateFacingTarget` (`self.GetAvatarActorFromActorInfo`) (`self.ProjectileTargetLocation`))
      (`AbilityTask_PlayMontageAndWait.CreatePlayMontageAndWaitProxy` "None" "/Game/Assets/Characters/Aura/Animations/Abilities/AM_Cast_FireBolt.AM_Cast_FireBolt" 1.0 "None" false
        (:`then`
          (`AbilityTask_WaitGameplayEvent.WaitGameplayEvent` (struct :`TagName` "Event.Montage.FireBolt") null
            (:`EventReceived`
              (bind _returnvalue (message `CombatInterface.GetCombatSocketLocation` (`self.GetAvatarActorFromActorInfo`) (`BlueprintGameplayTagLibrary.MakeLiteralGameplayTag` (struct :`TagName` "CombatSocket.Weapon"))))
              (`self.SpawnProjectile` (`self.ProjectileTargetLocation`) _returnvalue))))
        (:`OnCompleted`
          (`self.K2_EndAbility` :!label _label))
        (:`OnBlendOut`
          (goto _label))
        (:`OnInterrupted`
          (goto _label))
        (:`OnCancelled`
          (goto _label))))))