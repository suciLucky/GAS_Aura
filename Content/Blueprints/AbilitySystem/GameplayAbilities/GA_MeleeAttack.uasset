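; Gameplay ability that performs a melee attack with the goblin spear montage, turning the avatar toward its combat target first.
; A melee montage gameplay event triggers a small-radius search for live players around the combat socket, excluding the avatar.
; Actor tags restrict damage to the opposing Enemy or Player side.
; The ability ends after that hit check, or when the montage completes, is interrupted or is cancelled.
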(event `self.K2_ActivateAbility`
  (bind _returnvalue (`self.GetAvatarActorFromActorInfo`))
  (bind _returnvalue_2 (`self.GetAvatarActorFromActorInfo`))
  (bind _returnvalue_3 (message `EnemyInterface.GetCombatTarget` _returnvalue))
  (message `CombatInterface.UpdateFacingTarget` _returnvalue (`Actor.K2_GetActorLocation` _returnvalue_3))
  (`AbilityTask_PlayMontageAndWait.CreatePlayMontageAndWaitProxy` "None" "/Game/Assets/Enemies/Goblin/Animations/Spear/AM_Attack_GoblinSpear.AM_Attack_GoblinSpear"
    (:`then`
      (`AbilityTask_WaitGameplayEvent.WaitGameplayEvent` (struct :`TagName` "Event.Montage.Attack.Melee") null
        (:`EventReceived`
          (bind _returnvalue_4 (message `CombatInterface.GetCombatSocketLocation` _returnvalue_2))
          (bind _outoverlappingactors (`AuraAbilitySystemLibrary.GetLivePlayersInRadius` _returnvalue_2 (`|MakeArray` _returnvalue_2) 45.0 _returnvalue_4))
          (for _array_element _outoverlappingactors
            (if (`Actor.ActorHasTag` _returnvalue_2 "Enemy")
              (if (`Actor.ActorHasTag` _array_element "Player")
                (`self.CauseDamage` _array_element :!label _label))
              (elif (`Actor.ActorHasTag` _array_element "Enemy")
                (goto _label))))
          (`self.K2_EndAbility`))))
    (:`OnCompleted`
      (`self.K2_EndAbility` :!label _label_2))
    (:`OnInterrupted`
      (goto _label_2))
    (:`OnCancelled`
      (goto _label_2))))