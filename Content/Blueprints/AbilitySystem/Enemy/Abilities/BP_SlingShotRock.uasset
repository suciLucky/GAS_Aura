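; BP_SlingShotRock is the rock actor for an enemy slingshot ability, and its graph only handles the visual tumble.
; Each Tick adds a relative rotation to RockMesh, re-rolling a random rate of up to one turn per second on each axis and scaling it by delta time.
; The graph contains no movement, overlap or damage logic.
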(event `self.ReceiveTick`
  (params (DeltaSeconds :type "Float (single-precision)"))
  (`SceneComponent.K2_AddRelativeRotation` (`self.RockMesh`) (`KismetMathLibrary.MakeRotator` (* DeltaSeconds (* (`KismetMathLibrary.RandomFloat`) 360.0)) (* DeltaSeconds (* (`KismetMathLibrary.RandomFloat`) 360.0)) (* DeltaSeconds (* (`KismetMathLibrary.RandomFloat`) 360.0))) false false))

(fn `UserConstructionScript`)