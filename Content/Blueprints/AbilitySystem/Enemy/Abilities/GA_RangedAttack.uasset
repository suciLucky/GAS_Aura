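; Enemy ranged attack gameplay ability that fires a projectile at the avatar's combat target.
; On activation it turns the avatar toward the target and plays a random tagged attack montage from the avatar.
; The montage's gameplay event tag triggers SpawnProjectile from the combat socket matching that montage's socket tag, aimed at the target's location.
; The ability ends when the montage completes, is interrupted or is cancelled.
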(event `self.K2_ActivateAbility`
  (bind _returnvalue (`self.GetAvatarActorFromActorInfo`))
  (bind (_animmontage _montagetag _sockettag) (break `TaggedMontage` (`self.TaggedMontage`)))
  (bind _returnvalue_2 (message `EnemyInterface.GetCombatTarget` _returnvalue))
  (bind _returnvalue_3 (`Actor.K2_GetActorLocation` _returnvalue_2))
  (message `CombatInterface.UpdateFacingTarget` _returnvalue _returnvalue_3)
  (bind _returnvalue_4 (message `CombatInterface.GetAttackTaggedMontages` _returnvalue))
  (set `self.TaggedMontage` (`KismetArrayLibrary.Array_Random` _returnvalue_4))
  (`AbilityTask_PlayMontageAndWait.CreatePlayMontageAndWaitProxy` "None" _animmontage
    (:`then`
      (`AbilityTask_WaitGameplayEvent.WaitGameplayEvent` _montagetag null
        (:`EventReceived`
          (bind _returnvalue_5 (message `CombatInterface.GetCombatSocketLocation` (`self.GetAvatarActorFromActorInfo`) _sockettag))
          (`self.SpawnProjectile` _returnvalue_3 _returnvalue_5))))
    (:`OnCompleted`
      (`self.K2_EndAbility` :!label _label))
    (:`OnInterrupted`
      (goto _label))
    (:`OnCancelled`
      (goto _label))))