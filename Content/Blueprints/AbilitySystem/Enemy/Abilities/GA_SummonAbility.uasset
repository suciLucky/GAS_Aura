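; Enemy gameplay ability that summons random minions at shuffled spawn locations around a Shaman's attack.
; It faces the combat target, plays the fixed Shaman summon montage (the randomly picked tagged montage goes unused) and waits for its gameplay event.
; The event triggers ground Niagara effects, then a delayed loop spawns minions one by one, facing the summoner.
; Each spawn increments the summoner's minion count, and its destruction decrements it.
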(event `self.K2_ActivateAbility`
  (bind _returnvalue (`self.GetAvatarActorFromActorInfo`))
  (bind _returnvalue_2 (+ (`|GetArrayItem` (`self.SpawnLocations`) (`self.SpawnLocationIndex`)) (0.0 0.0 50.0)))
  (bind _returnvalue_3 (message `EnemyInterface.GetCombatTarget` _returnvalue))
  (message `CombatInterface.UpdateFacingTarget` _returnvalue (`Actor.K2_GetActorLocation` _returnvalue_3))
  (bind _returnvalue_4 (message `CombatInterface.GetAttackTaggedMontages` _returnvalue))
  (set `self.TaggedMontage` (`KismetArrayLibrary.Array_Random` _returnvalue_4))
  (`AbilityTask_PlayMontageAndWait.CreatePlayMontageAndWaitProxy` "None" "/Game/Assets/Enemies/Shaman/Animations/AM_Shaman_Summon.AM_Shaman_Summon"
    (:`then`
      (`AbilityTask_WaitGameplayEvent.WaitGameplayEvent` (struct :`TagName` "Montage.Attack.1") null
        (:`EventReceived`
          (bind _returnvalue_5 (`self.GetSpawnLocations`))
          (bind _output_get (set `self.SpawnLocations` _returnvalue_5))
          (`KismetArrayLibrary.Array_Shuffle` _output_get)
          (for _array_element _output_get
            (`NiagaraFunctionLibrary.SpawnSystemAtLocation` "/Game/Assets/Effects/Combat/NS_GroundSummon.NS_GroundSummon" _array_element))
          (`KismetSystemLibrary.Delay` 0.7)
          (if (< (`self.SpawnLocationIndex`) (`KismetArrayLibrary.Array_Length` (`self.SpawnLocations`))) :!label _label
            (bind _returnvalue_6 (`|SpawnActorFromClass` (`self.GetRandomMinionClass`) (`KismetMathLibrary.MakeTransform` _returnvalue_2 (`KismetMathLibrary.FindLookAtRotation` _returnvalue_2 (`Actor.K2_GetActorLocation` (`self.GetAvatarActorFromActorInfo`)))) "AlwaysSpawn" "MultiplyWithRoot" null null))
            (add `Actor.OnDestroyed` _returnvalue_6 (delegate `OnDestroyed_事件`))
            (message `CombatInterface.IncrementMinionCount` (`self.GetAvatarActorFromActorInfo`) 1)
            (`/Engine/EditorBlueprintResources/StandardMacros.IncrementInt` (`self.SpawnLocationIndex`)
              (:`  `
                (`KismetSystemLibrary.Delay` 0.2)
                (goto _label)))
            (else
              (set `self.SpawnLocationIndex` 0)
              (`self.K2_EndAbility`))))))
    (:`OnInterrupted`
      (set `self.SpawnLocationIndex` 0 :!label _label_2)
      (`self.K2_EndAbility`))
    (:`OnCancelled`
      (goto _label_2))))

(event `OnDestroyed_事件`
  (params (DestroyedActor :type "Actor Object Reference"))
  (message `CombatInterface.IncrementMinionCount` (`self.GetAvatarActorFromActorInfo`) -1))