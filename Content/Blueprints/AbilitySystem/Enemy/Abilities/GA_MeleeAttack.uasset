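; Enemy melee attack gameplay ability that turns toward the combat target and plays a random tagged attack montage.
; On the montage's gameplay event, it queries live players in a small radius around the montage's combat socket.
; Non-friendly hits take damage and spawn their own blood effect, with one MeleeImpact cue fired if anything was hit.
; The ability ends after the hit check or when the montage completes, is interrupted or is cancelled.
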(event `self.K2_ActivateAbility`
  (bind _returnvalue (`self.GetAvatarActorFromActorInfo`))
  (bind _returnvalue_2 (`self.GetAvatarActorFromActorInfo`))
  (bind (_animmontage _montagetag _sockettag) (break `TaggedMontage` (`self.TaggedMontage`)))
  (set `self.HasHitTarget` false)
  (bind _returnvalue_3 (message `EnemyInterface.GetCombatTarget` _returnvalue))
  (message `CombatInterface.UpdateFacingTarget` _returnvalue (`Actor.K2_GetActorLocation` _returnvalue_3))
  (bind _returnvalue_4 (message `CombatInterface.GetAttackTaggedMontages` _returnvalue))
  (set `self.TaggedMontage` (`KismetArrayLibrary.Array_Random` _returnvalue_4))
  (`AbilityTask_PlayMontageAndWait.CreatePlayMontageAndWaitProxy` "None" _animmontage
    (:`then`
      (`AbilityTask_WaitGameplayEvent.WaitGameplayEvent` _montagetag null
        (:`EventReceived`
          (bind _returnvalue_5 (message `CombatInterface.GetCombatSocketLocation` _returnvalue_2 _sockettag))
          (bind _outoverlappingactors (`AuraAbilitySystemLibrary.GetLivePlayersInRadius` _returnvalue_2 (`|MakeArray` _returnvalue_2) 45.0 _returnvalue_5))
          (for _array_element _outoverlappingactors
            (if (`AuraAbilitySystemLibrary.IsNotFriend` (`self.GetAvatarActorFromActorInfo`) _array_element)
              (`self.CauseDamage` _array_element)
              (set `self.HasHitTarget` true)
              (bind _returnvalue_6 (message `CombatInterface.GetBloodEffect` _array_element))
              (`NiagaraFunctionLibrary.SpawnSystemAtLocation` _returnvalue_6 _returnvalue_5)))
          (if (`self.HasHitTarget`)
            (`self.K2_ExecuteGameplayCueWithParams` (struct :`TagName` "GameplayCue.MeleeImpact") (`AbilitySystemBlueprintLibrary.MakeGameplayCueParameters` 0.0 0.0 (struct) (struct) (struct) (`BlueprintGameplayTagLibrary.MakeGameplayTagContainerFromTag` (`.MontageTag` (break `TaggedMontage` (`self.TaggedMontage`)))) (struct) _returnvalue_5 (0.0 0.0 0.0) null (`self.GetAvatarActorFromActorInfo`))))
          (`self.K2_EndAbility`))))
    (:`OnCompleted`
      (`self.K2_EndAbility` :!label _label))
    (:`OnInterrupted`
      (goto _label))
    (:`OnCancelled`
      (goto _label))))